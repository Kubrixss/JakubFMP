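; Black hole actor that periodically pulses, animating its scale with a timeline and playing a Pulse component alongside it.
; After a random initial delay it pulses, then has a roughly even chance of pulsing again immediately.
; Either way, a randomly timed cooldown blocks further chaining until it triggers the next pulse.
; A Reset event re-enters the initial delay.
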(event Custom|Reset
  (Utilities|FlowControl|Delay (Math|Random|RandomFloatinRange 15.0 3e+01))
  (Audio|Components|Audio|Play (Variables|Default|GetPulse) 0.0)
  (bind _newtrack_0 (Timeline|Timeline PlayFromStart)
    (:Update
      (Transformation|SetActorScale3D (Math|Conversions|ToVector(Float) _newtrack_0)))
    (:Finished
      (if (not (Variables|Default|GetCooldown))
        (if (> (Math|Random|RandomFloatinRange 0.0 2.0) 1.0)
          (CallFunction|PlayAgain)
          (CallFunction|CD)
          (else
            (CallFunction|CD)))))))

(event Custom|CD
  (Variables|Default|SetCooldown true)
  (Utilities|FlowControl|Delay (Math|Random|RandomFloatinRange 15.0 3e+01))
  (Variables|Default|SetCooldown false)
  (CallFunction|PlayAgain))

(event Custom|PlayAgain
  (Audio|Components|Audio|Play (Variables|Default|GetPulse) 0.0)
  (bind _newtrack_0 (Timeline|Timeline PlayFromStart)
    (:Update
      (Transformation|SetActorScale3D (Math|Conversions|ToVector(Float) _newtrack_0)))
    (:Finished
      (if (not (Variables|Default|GetCooldown))
        (if (> (Math|Random|RandomFloatinRange 0.0 2.0) 1.0)
          (CallFunction|PlayAgain)
          (CallFunction|CD)
          (else
            (CallFunction|CD)))))))

(event EventBeginPlay
  (Utilities|FlowControl|Delay (Math|Random|RandomFloatinRange 15.0 3e+01))
  (Audio|Components|Audio|Play (Variables|Default|GetPulse) 0.0)
  (bind _newtrack_0 (Timeline|Timeline PlayFromStart)
    (:Update
      (Transformation|SetActorScale3D (Math|Conversions|ToVector(Float) _newtrack_0)))
    (:Finished
      (if (not (Variables|Default|GetCooldown))
        (if (> (Math|Random|RandomFloatinRange 0.0 2.0) 1.0)
          (CallFunction|PlayAgain)
          (CallFunction|CD)
          (else
            (CallFunction|CD)))))))

(fn ConstructionScript)