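; GrabbableObject is a physical prop Blueprint with a cube mesh that plays impact sounds and a dissolve effect for despawning.
; DespawnDissolve runs a timeline that, on every update, creates dissolve material instances across the cube's material slots and drives their Progress parameter.
; Component hits above a speed threshold play a thud at the impact point, throttled by a DoOnce that resets after a short random delay.
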(event OnComponentHit(Cube)
  (params (HitComponent :type Primitive%20Component%20Object%20Reference) (OtherActor :type Actor%20Object%20Reference) (OtherComp :type Primitive%20Component%20Object%20Reference) (NormalImpulse :type Vector :default "0, 0, 0") (Hit :type Hit%20Result%20Structure%20%28by%20ref%29))
  (if (> (Math|Vector|VectorLength (Transformation|GetComponentVelocity (Variables|Default|GetCube))) 2e+01)
    (Utilities|FlowControl|Sequence
      (:then_0
        (Utilities|FlowControl|DoOnce false :!label _label
          (:Completed
            (Audio|PlaySoundatLocation "/Game/Audio/BoxThud.BoxThud" (.Location (Collision|BreakHitResult Hit)) "0, 0, 0" 1.0 1.0 0.0 "/Game/Audio/BoxThudA.BoxThudA" 0 0 0))))
      (:then_1
        (Utilities|FlowControl|Delay (Math|Random|RandomFloatinRange 0.1 0.2))
        (goto _label Reset)))))

(event Custom|DespawnDissolve
  (bind _newtrack_0 (Timeline|Timeline Play)
    (:Update
      (for _index (range 0 8)
        (bind _returnvalue (Rendering|Material|CreateDynamicMaterialInstance (Variables|Default|GetCube) _index "/Game/Material/M_Dissolve1.M_Dissolve1" "None" :!class /Script/Engine.PrimitiveComponent))
        (bind _output_get (Variables|Default|SetDynamic%20Material _returnvalue))
        (Rendering|Material|SetScalarParameterValue _output_get "Progress" _newtrack_0 :!class /Script/Engine.MaterialInstanceDynamic)))))

(fn ConstructionScript)

(fn OnRepElementIndex)