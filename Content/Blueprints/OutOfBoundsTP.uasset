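; Out-of-bounds trigger that teleports the player back to the nearest respawn point.
; BeginPlay seeds ClosestPoint with the first OutOfBoundsRespawnPoint actor in the level.
; When BP_FirstPersonCharacter overlaps OOBCollider, it loops through all respawn points, keeping the one closest to player 0.
; It then teleports player 0 to that point's full transform without sweeping.
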(event OnComponentBeginOverlap(OOBCollider)
  (params (OverlappedComponent :type Primitive%20Component%20Object%20Reference) (OtherActor :type Actor%20Object%20Reference) (OtherComp :type Primitive%20Component%20Object%20Reference) (OtherBodyIndex :type Integer) (bFromSweep :type Boolean) (SweepResult :type Hit%20Result%20Structure%20%28by%20ref%29))
  ;[1 1 1] Finds closest point and sets it
  (Utilities|Casting|CastToBP_FirstPersonCharacter OtherActor)
  (bind _outactors (Actor|GetAllActorsOfClass "/Game/Blueprints/OutOfBoundsRespawnPoint.OutOfBoundsRespawnPoint_C"))
  (for _array_element _outactors
    (if (< (Transformation|GetDistanceTo _array_element (Game|GetPlayerCharacter 0)) (Transformation|GetDistanceTo (Variables|Default|GetClosestPoint) (Game|GetPlayerCharacter 0)))
      (Variables|Default|SetClosestPoint _array_element)))
  (Transformation|SetActorTransform (Game|GetPlayerCharacter 0) (Transformation|GetActorTransform (Variables|Default|GetClosestPoint)) false true))

(event EventBeginPlay
  ;[1 1 1] Beginning value
  (bind _outactors (Actor|GetAllActorsOfClass "/Game/Blueprints/OutOfBoundsRespawnPoint.OutOfBoundsRespawnPoint_C"))
  (Variables|Default|SetClosestPoint (Utilities|Array|Get(acopy) _outactors)))

(fn ConstructionScript)