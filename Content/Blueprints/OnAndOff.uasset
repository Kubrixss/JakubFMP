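; Actor with two indicators that switch between on and off looks and can move vertically on a loop.
; The On and Off events swap the material on both indicators.
; If the On flag is set at BeginPlay, a timeline starts after a random sub-second delay and restarts whenever it finishes.
; Each update adds a Z world offset from the track value divided by a fresh random factor, so movement varies and depends on frame rate.
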(event Custom|Repeat
  (bind _newtrack_0 (Timeline|Timeline PlayFromStart)
    (:Update
      (Transformation|AddActorWorldOffset (Math|Vector|MakeVector 0.0 0.0 (/ _newtrack_0 (Math|Random|RandomFloatinRange 2.0 3.0)))))
    (:Finished
      (CallFunction|Repeat))))

(event Custom|Off
  (Rendering|Material|SetMaterial (Variables|Default|GetIndicator1) 0 (Variables|Default|GetMaterialOff)))

(event Custom|On
  (Rendering|Material|SetMaterial (Variables|Default|GetIndicator1) 0 (Variables|Default|GetMaterialOn)))

(event EventBeginPlay
  (if (Variables|Default|GetOn?)
    (Utilities|FlowControl|Delay (Math|Random|RandomFloatinRange 0.0 1.0))
    (bind _newtrack_0 (Timeline|Timeline Play)
      (:Update
        (Transformation|AddActorWorldOffset (Math|Vector|MakeVector 0.0 0.0 (/ _newtrack_0 (Math|Random|RandomFloatinRange 2.0 3.0)))))
      (:Finished
        (CallFunction|Repeat)))))

(fn ConstructionScript)