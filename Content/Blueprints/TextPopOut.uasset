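; TextPopOut is a world info label that shows configurable text through an InfoPanel widget and fades it by the player's distance.
; The first-person character entering the box starts a fast looping timer, presumably bound to OpacityCheck.
; OpacityCheck keeps the text opaque within MaxVisDistance and fades it linearly over a fixed band beyond.
; Leaving the box clears the timer and hides the text.
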(event OnComponentBeginOverlap(Box)
  (params (OverlappedComponent :type Primitive%20Component%20Object%20Reference) (OtherActor :type Actor%20Object%20Reference) (OtherComp :type Primitive%20Component%20Object%20Reference) (OtherBodyIndex :type Integer) (bFromSweep :type Boolean) (SweepResult :type Hit%20Result%20Structure%20%28by%20ref%29))
  (Utilities|Casting|CastToBP_FirstPersonCharacter OtherActor)
  (bind _returnvalue (Utilities|Time|SetTimerbyEvent (EventDispatchers|CreateEvent :!event Custom|OpacityCheck) 0.01 true)))

(event OnComponentEndOverlap(Box)
  (params (OverlappedComponent :type Primitive%20Component%20Object%20Reference) (OtherActor :type Actor%20Object%20Reference) (OtherComp :type Primitive%20Component%20Object%20Reference) (OtherBodyIndex :type Integer))
  (Utilities|Casting|CastToBP_FirstPersonCharacter OtherActor)
  (Utilities|Time|ClearandInvalidateTimerbyHandle (stale OnComponentBeginOverlap(Box) _returnvalue))
  (Widget|SetRenderOpacity (Variables|/Game/Blueprints/UI/InfoPanel.InfoPanel_C|GetTextBlock_0 (Variables|Default|GetAs%20Info%20Panel)) 0.0))

(event Custom|OpacityCheck
  (bind _self self)
  (bind _as_info_panel (Variables|Default|GetAs%20Info%20Panel))
  (bind _as_bp_first_person_character (Variables|Default|GetAs%20BP%20First%20Person%20Character))
  (bind _maxvisdistance (Variables|Default|GetMaxVisDistance))
  (bind _returnvalue (Transformation|GetDistanceTo _as_bp_first_person_character _self))
  (bind _textblock_0 (Variables|/Game/Blueprints/UI/InfoPanel.InfoPanel_C|GetTextBlock_0 _as_info_panel))
  (if (< _returnvalue _maxvisdistance)
    (Widget|SetRenderOpacity _textblock_0 1.0)
    (else
      (Widget|SetRenderOpacity _textblock_0 (Math|Float|Clamp(Float) (- 1.0 (/ (- _returnvalue _maxvisdistance) 2.5e+02)))))))

(event EventBeginPlay
  (bind _asinfo_panel (Utilities|Casting|CastToInfoPanel (UserInterface|GetWidget (Variables|Default|GetWidget))))
  (bind _output_get (Variables|Default|SetAs%20Info%20Panel _asinfo_panel))
  (Rendering|Components|TextRender|SetText (Variables|/Game/Blueprints/UI/InfoPanel.InfoPanel_C|GetTextBlock_0 _output_get) (Variables|Default|GetTextInput))
  (bind _asbp_first_person_character (Utilities|Casting|CastToBP_FirstPersonCharacter (Game|Player|GetPlayerPawn 0)))
  (Variables|Default|SetAs%20BP%20First%20Person%20Character _asbp_first_person_character))

(fn ConstructionScript)