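; A puzzle platform that the player drags along a spline by holding right mouse while aiming at it from inside its input trigger.
; Camera traces feed looping timers that lerp the platform toward the spline point nearest the aim, with a cable shown while held and movement timeout delayed after release.
; A completion collider fires configurable named functions, such as sliding door or platform re-enabling, while a stop collider halts movement.
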(event OnComponentBeginOverlap(CompletedCollider)
  (params (OverlappedComponent :type Primitive%20Component%20Object%20Reference) (OtherActor :type Actor%20Object%20Reference) (OtherComp :type Primitive%20Component%20Object%20Reference) (OtherBodyIndex :type Integer) (bFromSweep :type Boolean) (SweepResult :type Hit%20Result%20Structure%20%28by%20ref%29))
  (if (Class|PrimitiveComponent|IsOverlappingComponent (Variables|Default|GetMovingObject) (Variables|Default|GetCompletedCollider))
    (Utilities|Time|SetTimerbyFunctionName 0 (Variables|Default|GetOpenFunctionName) 0.001)
    (Utilities|Time|SetTimerbyFunctionName 0 (Variables|Default|GetReenableName) 0.001)))

(event OnComponentEndOverlap(CompletedCollider)
  (params (OverlappedComponent :type Primitive%20Component%20Object%20Reference) (OtherActor :type Actor%20Object%20Reference) (OtherComp :type Primitive%20Component%20Object%20Reference) (OtherBodyIndex :type Integer))
  (if (not (Class|PrimitiveComponent|IsOverlappingComponent (Variables|Default|GetMovingObject) (Variables|Default|GetCompletedCollider)))
    (Utilities|Time|SetTimerbyFunctionName 0 (Variables|Default|GetClosedFunctionName) 0.001)))

(event OnComponentBeginOverlap(StopCollider)
  (params (OverlappedComponent :type Primitive%20Component%20Object%20Reference) (OtherActor :type Actor%20Object%20Reference) (OtherComp :type Primitive%20Component%20Object%20Reference) (OtherBodyIndex :type Integer) (bFromSweep :type Boolean) (SweepResult :type Hit%20Result%20Structure%20%28by%20ref%29))
  (if (Class|PrimitiveComponent|IsOverlappingComponent (Variables|Default|GetMovingObject) (Variables|Default|GetStopCollider))
    (Utilities|FlowControl|DoOnce false
      (:Completed
        (Variables|Default|SetLerpAmount 0.0)
        (Utilities|Time|ClearandInvalidateTimerbyHandle (stale Custom|MovingAlongSpline _returnvalue))))))

(event OnComponentBeginOverlap(Enables/DisablesInputCollider)
  (params (OverlappedComponent :type Primitive%20Component%20Object%20Reference) (OtherActor :type Actor%20Object%20Reference) (OtherComp :type Primitive%20Component%20Object%20Reference) (OtherBodyIndex :type Integer) (bFromSweep :type Boolean) (SweepResult :type Hit%20Result%20Structure%20%28by%20ref%29))
  (Utilities|Casting|CastToBP_FirstPersonCharacter OtherActor)
  (Input|EnableInput (Game|GetPlayerController 0)))

(event OnComponentEndOverlap(Enables/DisablesInputCollider)
  (params (OverlappedComponent :type Primitive%20Component%20Object%20Reference) (OtherActor :type Actor%20Object%20Reference) (OtherComp :type Primitive%20Component%20Object%20Reference) (OtherBodyIndex :type Integer))
  (Utilities|Casting|CastToBP_FirstPersonCharacter OtherActor)
  (Input|DisableInput (Game|GetPlayerController 0))
  (Rendering|SetVisibility (Variables|Default|GetCable) false false)
  (Variables|Default|SetIsHoldingLMB false)
  (Variables|Default|SetLookingAtPlatform false)
  ;[1 1 1] Looking At Platform
  (CallFunction|ResetDoOnce)
  (Utilities|Time|ClearandInvalidateTimerbyHandle (stale Input|MouseEvents|RightMouseButton _returnvalue_2))
  (Utilities|FlowControl|RetriggerableDelay 5.0)
  (Utilities|Time|ClearandInvalidateTimerbyHandle (stale Custom|MovingAlongSpline _returnvalue)))

(event Custom|MovingAlongSpline
  ;[1 1 1] Moving Along Spline
  (if (Variables|Default|GetLookingAtPlatform)
    (bind _asbp_first_person_character (Utilities|Casting|CastToBP_FirstPersonCharacter (Game|GetPlayerCharacter 0)))
    (bind _outhit (Collision|LineTraceByChannel (Transformation|GetWorldLocation (Variables|/Game/FirstPerson/Blueprints/BP_FirstPersonCharacter.BP_FirstPersonCharacter_C|GetFirstPersonCamera _asbp_first_person_character)) (+ (* (Math|Vector|GetForwardVector (Variables|/Game/FirstPerson/Blueprints/BP_FirstPersonCharacter.BP_FirstPersonCharacter_C|GetFirstPersonCamera _asbp_first_person_character)) 1.5e+03) (Transformation|GetWorldLocation (Variables|/Game/FirstPerson/Blueprints/BP_FirstPersonCharacter.BP_FirstPersonCharacter_C|GetFirstPersonCamera _asbp_first_person_character))) "TraceTypeQuery1" false 0 "None"))
    (if (.bBlockingHit (Collision|BreakHitResult _outhit))
      (Utilities|FlowControl|DoOnce false
        (:Completed
          (bind _returnvalue (Utilities|Time|SetTimerbyEvent (delegate Custom|Moving) 0.001 true)))))))

(event Custom|Moving
  (bind _movingobject (Variables|Default|GetMovingObject))
  ;[1 1 1] Moving Along Spline
  (if (.bBlockingHit (Collision|BreakHitResult (stale Custom|MovingAlongSpline _outhit)))
    (Transformation|SetWorldTransform _movingobject (Math|Transform|MakeTransform (Math|Vector|Lerp(Vector) (Transformation|GetWorldLocation _movingobject) (Spline|FindLocationClosesttoWorldLocation (Variables|Default|GetSpline) (.Location (Collision|BreakHitResult (stale Custom|MovingAlongSpline _outhit))) "World") (Variables|Default|GetLerpAmount)) "0, 0, 0" "1.000000,1.000000,1.000000") false false)
    (Variables|/Script/CableComponent.CableComponent|SetEndLocation (Variables|Default|GetCable) (Math|Transform|InverseTransformLocation (Transformation|GetActorTransform) (Transformation|GetActorLocation (Game|Player|GetPlayerPawn 0))))))

(event Custom|ResetDoOnce
  ;[1 1 1] Moving Along Spline
  (Utilities|FlowControl|DoOnce false) ; enters at Reset
)

(event EventBeginPlay
  (Transformation|SetWorldTransform (Variables|Default|GetMovingObject) (Math|Transform|MakeTransform (.location (Spline|GetTransformatDistanceAlongSpline (Variables|Default|GetSpline) 0.0 "World" false)) "0, 0, 0" "1.000000,1.000000,1.000000") false false))

(event EventTick
  (params (DeltaSeconds :type Float%20%28single-precision%29))
  ;[1 1 1] TIck
)

(event Input|MouseEvents|RightMouseButton
  (params (Key :type Key%20Structure :default "None"))
  ;[1 1 1] Looking At Platform
  (:Pressed
    (Variables|Default|SetIsHoldingLMB true)
    (bind _asbp_first_person_character (Utilities|Casting|CastToBP_FirstPersonCharacter (Game|GetPlayerCharacter 0)))
    (bind (_outhit _returnvalue) (Collision|LineTraceByChannel (Transformation|GetWorldLocation (Variables|/Game/FirstPerson/Blueprints/BP_FirstPersonCharacter.BP_FirstPersonCharacter_C|GetFirstPersonCamera _asbp_first_person_character)) (+ (* (Math|Vector|GetForwardVector (Variables|/Game/FirstPerson/Blueprints/BP_FirstPersonCharacter.BP_FirstPersonCharacter_C|GetFirstPersonCamera _asbp_first_person_character)) (Math|Vector|MakeVector 1e+03 1e+03 1e+03)) (Transformation|GetWorldLocation (Variables|/Game/FirstPerson/Blueprints/BP_FirstPersonCharacter.BP_FirstPersonCharacter_C|GetFirstPersonCamera _asbp_first_person_character))) "TraceTypeQuery1" false 0 "None" false))
    (if _returnvalue
      (if (== (Variables|Default|GetMovingObject) (.HitComponent (Collision|BreakHitResult _outhit)))
        (if (.bBlockingHit (Collision|BreakHitResult _outhit))
          (Variables|Default|SetLookingAtPlatform true)
          (bind _returnvalue_2 (Utilities|Time|SetTimerbyEvent (delegate Custom|MovingAlongSpline) 0.01 true))
          (Rendering|SetVisibility (Variables|Default|GetCable) true false))
        (else
          (Variables|Default|SetLookingAtPlatform false :!label _label)))
      (else
        (goto _label))))
  (:Released
    (Rendering|SetVisibility (Variables|Default|GetCable) false false)
    (Variables|Default|SetIsHoldingLMB false)
    (Variables|Default|SetLookingAtPlatform false)
    (CallFunction|ResetDoOnce)
    (Utilities|Time|ClearandInvalidateTimerbyHandle _returnvalue_2)
    (Utilities|FlowControl|RetriggerableDelay 5.0)
    (Utilities|Time|ClearandInvalidateTimerbyHandle (stale Custom|MovingAlongSpline _returnvalue))))

(fn ConstructionScript)

(fn TestFunctionOpening
  (bind _outactors (Actor|GetAllActorsOfClasswithTag "/Game/Blueprints/SlidingDoor.SlidingDoor_C" "Door1"))
  (bind _output_get (Variables|Default|SetOpeningDoor (Utilities|Array|Get(acopy) _outactors)))
  (Default|Activated _output_get))

(fn TestFunctionClosing
  (Default|Deactivated (Variables|Default|GetOpeningDoor)))

(fn Re-EnableDoor
  (Development|PrintString "Hello")
  (bind _outactors (Actor|GetAllActorsOfClasswithTag "MovingPlatformRed_C" "Puzzle1"))
  (bind _output_get (Variables|Default|SetMovingPlatform (Utilities|Array|Get(acopy) _outactors)))
  (Variables|MovingPlatformRed_C|SetLerpAmount _output_get 0.001))