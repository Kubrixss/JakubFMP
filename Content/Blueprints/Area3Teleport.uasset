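; Area3Teleport is a trigger Blueprint that sends the player to the Area3 level when BP_FirstPersonCharacter overlaps its Box.
; It compares the character's Minutes and Seconds, converted to total seconds, with the Level2 time in JakubGameInstance, overwriting the stored time only if the character's is greater.
; It then shows the LoadingScreenArea3 widget and opens the level after a short delay.
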(event OnComponentBeginOverlap(Box)
  (params (OverlappedComponent :type Primitive%20Component%20Object%20Reference) (OtherActor :type Actor%20Object%20Reference) (OtherComp :type Primitive%20Component%20Object%20Reference) (OtherBodyIndex :type Integer) (bFromSweep :type Boolean) (SweepResult :type Hit%20Result%20Structure%20%28by%20ref%29))
  (bind _asbp_first_person_character (Utilities|Casting|CastToBP_FirstPersonCharacter OtherActor))
  (bind _asjakub_game_instance (Utilities|Casting|CastToJakubGameInstance (Game|GetGameInstance)))
  (if (> (+ (* (Variables|/Game/FirstPerson/Blueprints/BP_FirstPersonCharacter.BP_FirstPersonCharacter_C|GetMinutes _asbp_first_person_character) 6e+01) (Variables|/Game/FirstPerson/Blueprints/BP_FirstPersonCharacter.BP_FirstPersonCharacter_C|GetSeconds _asbp_first_person_character)) (+ (* (Variables|/Game/Blueprints/JakubGameInstance.JakubGameInstance_C|GetLevel2Minutes _asjakub_game_instance) 6e+01) (Variables|/Game/Blueprints/JakubGameInstance.JakubGameInstance_C|GetLevel2Seconds _asjakub_game_instance)))
    (Variables|/Game/Blueprints/JakubGameInstance.JakubGameInstance_C|SetLevel2Minutes _asjakub_game_instance (Variables|/Game/FirstPerson/Blueprints/BP_FirstPersonCharacter.BP_FirstPersonCharacter_C|GetMinutes _asbp_first_person_character))
    (Variables|/Game/Blueprints/JakubGameInstance.JakubGameInstance_C|SetLevel2Seconds _asjakub_game_instance (Variables|/Game/FirstPerson/Blueprints/BP_FirstPersonCharacter.BP_FirstPersonCharacter_C|GetSeconds _asbp_first_person_character)))
  (bind _returnvalue (UserInterface|CreateWidget "/Game/Blueprints/UI/LoadingScreenArea3.LoadingScreenArea3_C" (Game|GetPlayerController 0)))
  (UserInterface|Viewport|AddtoViewport _returnvalue 0)
  (Utilities|FlowControl|Delay 0.2)
  (Game|OpenLevel(byName) "Area3"))

(event EventBeginPlay)

(event Collision|EventActorBeginOverlap
  (params (OtherActor :type Actor%20Object%20Reference)))

(event EventTick
  (params (DeltaSeconds :type Float%20%28single-precision%29)))

(fn ConstructionScript)