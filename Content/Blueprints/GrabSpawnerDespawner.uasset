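; A spawner actor that keeps a grabbable cube available and lets the player reset it.
; It spawns a GrabbableObject at CubeSpawnLocation on BeginPlay, and Tick spawns a replacement whenever that object becomes invalid.
; An overlap volume enables input only while the first-person character is inside.
; Pressing Interact runs a short camera line trace; hitting the Sphere component destroys the current cube and spawns a new one.
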(event OnComponentBeginOverlap(Enable/DisableInput)
  (params (OverlappedComponent :type Primitive%20Component%20Object%20Reference) (OtherActor :type Actor%20Object%20Reference) (OtherComp :type Primitive%20Component%20Object%20Reference) (OtherBodyIndex :type Integer) (bFromSweep :type Boolean) (SweepResult :type Hit%20Result%20Structure%20%28by%20ref%29))
  (Utilities|Casting|CastToBP_FirstPersonCharacter OtherActor)
  (Input|EnableInput (Game|GetPlayerController 0)))

(event OnComponentEndOverlap(Enable/DisableInput)
  (params (OverlappedComponent :type Primitive%20Component%20Object%20Reference) (OtherActor :type Actor%20Object%20Reference) (OtherComp :type Primitive%20Component%20Object%20Reference) (OtherBodyIndex :type Integer))
  (Utilities|Casting|CastToBP_FirstPersonCharacter OtherActor)
  (Input|DisableInput (Game|GetPlayerController 0)))

(event Custom|DespawnCube
  (Utilities|IsValid (stale Custom|SpawnCube _returnvalue)
    (:Is%20Valid
      (Actor|DestroyActor (stale Custom|SpawnCube _returnvalue))
      (CallFunction|SpawnCube))
    (:Is%20Not%20Valid
      (CallFunction|SpawnCube))))

(event Custom|SpawnCube
  (bind _returnvalue (Game|SpawnActorfromClass "/Game/Blueprints/GrabbableObject.GrabbableObject_C" (Transformation|GetWorldTransform (Variables|Default|GetCubeSpawnLocation)) "Undefined" "MultiplyWithRoot" 0 0))
  (Variables|Default|SetCubeRef _returnvalue))

(event EventBeginPlay
  (CallFunction|SpawnCube)
  (bind _returnvalue (Actor|GetActorOfClass "/Game/FirstPerson/Blueprints/BP_FirstPersonCharacter.BP_FirstPersonCharacter_C"))
  (Variables|Default|SetPlayerRef _returnvalue))

(event EventTick
  (params (DeltaSeconds :type Float%20%28single-precision%29))
  (Utilities|IsValid (stale Custom|SpawnCube _returnvalue)
    (:Is%20Not%20Valid
      (CallFunction|SpawnCube))))

(event Input|ActionEvents|InputActionInteract
  (params (Key :type Key%20Structure :default "None"))
  (bind _playerref (Variables|Default|GetPlayerRef))
  (bind _firstpersoncamera (Variables|/Game/FirstPerson/Blueprints/BP_FirstPersonCharacter.BP_FirstPersonCharacter_C|GetFirstPersonCamera _playerref))
  (bind _returnvalue (Transformation|GetWorldLocation _firstpersoncamera))
  (:Pressed
    (bind _outhit (Collision|LineTraceByChannel _returnvalue (+ _returnvalue (* (Math|Vector|GetForwardVector (Transformation|GetWorldRotation _firstpersoncamera)) 2e+02)) "TraceTypeQuery1" false 0 "None" false))
    (if (== (Variables|Default|GetSphere) (.HitComponent (Collision|BreakHitResult _outhit)))
      (CallFunction|DespawnCube))))

(fn ConstructionScript)